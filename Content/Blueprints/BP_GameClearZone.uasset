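; BP_GameClearZone is a trigger zone that tracks whether the player stands where they can escape, presumably to clear the game.
; Box overlap events compare the other actor with a stored player reference, setting CanEscape on entry and clearing it on exit.
; The cast that would store that reference is disconnected and BeginPlay is empty, so this graph never assigns it.
; Nothing here acts on CanEscape.
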(event OnComponentBeginOverlap(Box)
  (params (OverlappedComponent :type Primitive%20Component%20Object%20Reference) (OtherActor :type Actor%20Object%20Reference) (OtherComp :type Primitive%20Component%20Object%20Reference) (OtherBodyIndex :type Integer) (bFromSweep :type Boolean) (SweepResult :type Hit%20Result%20Structure%20%28by%20ref%29))
  (if (== OtherActor (Variables|Default|GetAs%20BP%20Player))
    (Variables|Default|SetbCanEscape true)))

(event OnComponentEndOverlap(Box)
  (params (OverlappedComponent :type Primitive%20Component%20Object%20Reference) (OtherActor :type Actor%20Object%20Reference) (OtherComp :type Primitive%20Component%20Object%20Reference) (OtherBodyIndex :type Integer))
  (if (== (Variables|Default|GetAs%20BP%20Player) OtherActor)
    (Variables|Default|SetbCanEscape false)))

(event EventBeginPlay)

(fn ConstructionScript)