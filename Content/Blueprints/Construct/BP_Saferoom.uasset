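; Saferoom actor with a swinging door that the player opens and closes, triggering an escape attempt when it shuts with them in the escape zone.
; It binds Use to the player's use dispatcher and acts only while the player overlaps the door trigger.
; One timeline, played forward or in reverse, drives door yaw, with a pending flag guarding against re-triggering.
; When it finishes closed inside the escape zone, TryEscape is called.
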(event OnComponentBeginOverlap(DoorUse)
  (params (OverlappedComponent :type Primitive%20Component%20Object%20Reference) (OtherActor :type Actor%20Object%20Reference) (OtherComp :type Primitive%20Component%20Object%20Reference) (OtherBodyIndex :type Integer) (bFromSweep :type Boolean) (SweepResult :type Hit%20Result%20Structure%20%28by%20ref%29))
  ;[0.15 0.15 0.15 0.5] 플레이어가 근처에 있을때만 문 상호작용
  (if (== OtherActor (Variables|Default|GetAs%20BP%20Player))
    (Variables|Default|SetbPlayerIsNearby true)))

(event OnComponentEndOverlap(DoorUse)
  (params (OverlappedComponent :type Primitive%20Component%20Object%20Reference) (OtherActor :type Actor%20Object%20Reference) (OtherComp :type Primitive%20Component%20Object%20Reference) (OtherBodyIndex :type Integer))
  ;[0.15 0.15 0.15 0.5] 플레이어가 근처에 있을때만 문 상호작용
  (if (== (Variables|Default|GetAs%20BP%20Player) OtherActor)
    (Variables|Default|SetbPlayerIsNearby false)))

(event OnComponentBeginOverlap(EscapeZone)
  (params (OverlappedComponent :type Primitive%20Component%20Object%20Reference) (OtherActor :type Actor%20Object%20Reference) (OtherComp :type Primitive%20Component%20Object%20Reference) (OtherBodyIndex :type Integer) (bFromSweep :type Boolean) (SweepResult :type Hit%20Result%20Structure%20%28by%20ref%29))
  ;[0.15 0.15 0.15 0.5] 문이 닫혀있고 탈출구역 안에 있다면 탈출시도
  (if (== OtherActor (Variables|Default|GetAs%20BP%20Player))
    (Variables|Default|SetbCanEscape true)))

(event OnComponentEndOverlap(EscapeZone)
  (params (OverlappedComponent :type Primitive%20Component%20Object%20Reference) (OtherActor :type Actor%20Object%20Reference) (OtherComp :type Primitive%20Component%20Object%20Reference) (OtherBodyIndex :type Integer))
  ;[0.15 0.15 0.15 0.5] 문이 닫혀있고 탈출구역 안에 있다면 탈출시도
  (if (== (Variables|Default|GetAs%20BP%20Player) OtherActor)
    (Variables|Default|SetbCanEscape false)))

(event Custom|Use
  (if (Variables|Default|GetbPlayerIsNearby)
    (if (Variables|Default|GetbIsOpen)
      (CallFunction|Close)
      (else
        (CallFunction|Open)))))

(event Custom|Open
  ;[0.15 0.15 0.15 0.5] 문 열고닫기
  (if (Utilities|CanOpen)
    (Variables|Default|SetbIsPending true)
    (bind _openclose (Timeline|TL_OpenClose PlayFromStart)
      (:Update
        (Transformation|SetRelativeRotation (Variables|Default|GetSM_Door_3) (Math|Rotator|MakeRotator 0.0 0.0 (+ (Variables|Default|GetDoorStartOffset) (* _openclose (Variables|Default|GetOpenWidth)))) false false))
      (:Finished
        (Variables|Default|SetbIsPending false)
        (Variables|Default|SetbIsOpen (not (Variables|Default|GetbIsOpen)))
        ;[0.15 0.15 0.15 0.5] 탈출체크
        (if (and (Variables|Default|GetbCanEscape) (not (Variables|Default|GetbIsOpen)))
          (Default|CallTryEscape))))))

(event Custom|Close
  ;[0.15 0.15 0.15 0.5] 문 열고닫기
  (if (Utilities|CanClose)
    (Variables|Default|SetbIsPending true)
    (bind _openclose (Timeline|TL_OpenClose ReverseFromEnd)
      (:Update
        (Transformation|SetRelativeRotation (Variables|Default|GetSM_Door_3) (Math|Rotator|MakeRotator 0.0 0.0 (+ (Variables|Default|GetDoorStartOffset) (* _openclose (Variables|Default|GetOpenWidth)))) false false))
      (:Finished
        (Variables|Default|SetbIsPending false)
        (Variables|Default|SetbIsOpen (not (Variables|Default|GetbIsOpen)))
        ;[0.15 0.15 0.15 0.5] 탈출체크
        (if (and (Variables|Default|GetbCanEscape) (not (Variables|Default|GetbIsOpen)))
          (Default|CallTryEscape))))))

(event EventBeginPlay
  (Variables|Default|SetDoorStartOffset (.pitch (Variables|/Script/Engine.SceneComponent|GetRelativeRotation (Variables|Default|GetSM_Door_3))))
  (bind _asbp_player (Utilities|Casting|CastToBP_Player (Game|GetPlayerCharacter 0)))
  (bind _output_get (Variables|Default|SetAs%20BP%20Player _asbp_player))
  (EventDispatchers|AssignTryUseSomething _output_get (delegate Custom|Use)))

(fn ConstructionScript)