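; Wave-mode zombie character that hunts the player and attacks in melee.
; Chase re-issues AIMoveTo every 0.2 seconds at a random speed; on success, a DoOnce-gated Attack changes speed and, after a short delay, line-traces forward to damage the player and notify the HUD.
; Incoming damage sets a temporary stun flag before resuming the chase, or at the dying threshold ragdolls the mesh with a head impulse, then destroys the actor.
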(event Custom|Chase
  (bind _returnvalue (Transformation|GetActorLocation))
  (bind _returnvalue_2 (Game|GetPlayerCharacter 0))
  (Variables|Default|SetbDoAttack false)
  (Variables|/Script/Engine.CharacterMovementComponent|SetMaxWalkSpeed (Variables|Character|GetCharacterMovement) (Math|Random|RandomFloatinRange 4.5e+02 6.5e+02))
  (AI|AIMoveTo self "0, 0, 0" (Game|GetPlayerCharacter 0) 5.0 false
    (:then
      (Utilities|FlowControl|Delay 0.2)
      (CallFunction|Chase))
    (:OnSuccess
      (CallFunction|Attack)
      (Utilities|FlowControl|DoOnce false) ; enters at Reset
    )
    (:OnFail
      (CallFunction|Chase))))

(event Custom|Attack
  (bind _returnvalue (Transformation|GetActorLocation))
  (bind _returnvalue_2 (Game|GetPlayerCharacter 0))
  (Variables|Default|SetbDoAttack true)
  (Variables|/Script/Engine.CharacterMovementComponent|SetMaxWalkSpeed (Variables|Character|GetCharacterMovement) (Variables|Default|GetAttackWalkSpeed))
  (Utilities|FlowControl|DoOnce false
    (:Completed
      (Utilities|FlowControl|Delay 0.5)
      (bind _outhit (Collision|LineTraceByChannel _returnvalue (+ _returnvalue (* (Transformation|GetActorForwardVector) 1.5e+02)) "TraceTypeQuery1" false 0 "Persistent"))
      (if (== _returnvalue_2 (.hitactor _outhit))
        (if (not (<= (Variables|Default|GetZombieCurrentHealth) 0.0))
          (Game|Damage|ApplyDamage _returnvalue_2 (Math|Random|RandomFloatinRange (Variables|Default|GetMinDamage) (Variables|Default|GetMaxDamage)) 0 0)
          (bind _returnvalue_3 (Actor|GetActorOfClass "/Game/UI/HUD_HUD.HUD_HUD_C"))
          (Default|PlayerHit _returnvalue_3)
          (Utilities|FlowControl|Delay 1.5)
          (CallFunction|Chase))
        (else
          (CallFunction|Chase))))))

(event Game|Damage|EventAnyDamage
  (params (Damage :type Float%20%28single-precision%29) (DamageType :type Damage%20Type%20Object%20Reference) (InstigatedBy :type Controller%20Object%20Reference) (DamageCauser :type Actor%20Object%20Reference))
  (bind _mesh (Variables|Character|GetMesh))
  (bind _output_get (Variables|Default|SetZombieCurrentHealth (- (Variables|Default|GetZombieCurrentHealth) Damage)))
  (if (<= _output_get (Variables|Default|GetZombieDyingHealth))
    (Collision|SetCollisionProfileName _mesh "Ragdoll" true :!class /Script/Engine.PrimitiveComponent)
    (Physics|SetSimulatePhysics _mesh true)
    (Physics|AddImpulse (Variables|Character|GetMesh) "50000.000000,0.000000,0.000000" "head" false)
    (Collision|SetCollisionEnabled (Variables|Collision|GetCapsuleComponent) "NoCollision")
    (Utilities|FlowControl|Delay 5.0)
    (Actor|DestroyActor)
    (else
      (Variables|Default|SetbTakeDamage true)
      (Utilities|FlowControl|Delay (Variables|Default|GetTakeDamageStunTime))
      (Variables|Default|SetbTakeDamage false)
      (CallFunction|Chase))))

(event EventBeginPlay
  (CallFunction|Chase))

(fn ConstructionScript)