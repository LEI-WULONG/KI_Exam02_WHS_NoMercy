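; Zombie enemy that wanders to random nearby points until it hears or sees the player, then runs after them.
; Hearing (PawnSensing), sight (AIPerception) and non-lethal damage, after a brief stun, all feed Chase.
; Reaching the player triggers a slowed attack with a delayed forward line trace that applies random damage, notifies the HUD and resumes chasing.
; At the dying health threshold it ragdolls and is destroyed after a delay.
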(event OnTargetPerceptionUpdated(AIPerception_Sight)
  (params (Actor :type Actor%20Object%20Reference) (Stimulus :type AI%20Stimulus%20Structure))
  ;[0.15 0.15 0.15 0.5] 좀비가 플레이어를 발견했을 시
  (bind _output_get (Variables|Default|SetItMustBePlayer Actor))
  (if (== _output_get (Game|GetPlayerCharacter 0))
    (CallFunction|Chase)))

(event OnHearNoise(PawnSensing)
  (params (Instigator :type Pawn%20Object%20Reference) (Location :type Vector%20%28by%20ref%29 :default "0, 0, 0") (Volume :type Float%20%28single-precision%29))
  ;[0.15 0.15 0.15 0.5] 좀비가 플레이어의 소리를 들었을 시
  (Utilities|Casting|CastToBP_Player Instigator)
  (CallFunction|Chase))

(event Custom|Stray
  ;[0.15 0.15 0.15 0.5] 기본적으로 아무런 자극이 없을 경우 방황
  (AI|AIMoveTo self (.RandomLocation (AI|Navigation|GetRandomReachablePointinRadius (Transformation|GetActorLocation) 5e+02 0 0)) 0 5.0 false
    (:then
      (Utilities|FlowControl|Delay 5.0 :!label _label))
    (:OnSuccess
      (goto _label))
    (:OnFail
      _))
  (CallFunction|Stray))

(event Custom|Chase
  ;[0.15 0.15 0.15 0.5] 플레이어 추격 후 공격
  (Variables|Default|SetbDoAttack false)
  (Variables|/Script/Engine.CharacterMovementComponent|SetMaxWalkSpeed (Variables|Character|GetCharacterMovement) (Variables|Default|GetRunSpeed))
  (AI|AIMoveTo self "0, 0, 0" (Game|GetPlayerCharacter 0) 5.0 false
    (:OnSuccess
      (CallFunction|Attack)
      ;[0.15 0.15 0.15 0.5] 좀비 공격
      (Utilities|FlowControl|DoOnce false) ; enters at Reset
    )
    (:OnFail
      (CallFunction|Chase))))

(event Custom|Attack
  ;[0.15 0.15 0.15 0.5] 좀비 공격
  (Variables|Default|SetbDoAttack true)
  (Variables|/Script/Engine.CharacterMovementComponent|SetMaxWalkSpeed (Variables|Character|GetCharacterMovement) (Variables|Default|GetAttackWalkSpeed))
  (Utilities|FlowControl|DoOnce false
    (:Completed
      (Utilities|ZombieAttckModify))))

(event EventBeginPlay
  ;[0.15 0.15 0.15 0.5] 기본적으로 아무런 자극이 없을 경우 방황
  (CallFunction|Stray))

(event Game|Damage|EventAnyDamage
  (params (Damage :type Float%20%28single-precision%29) (DamageType :type Damage%20Type%20Object%20Reference) (InstigatedBy :type Controller%20Object%20Reference) (DamageCauser :type Actor%20Object%20Reference))
  ;[0.15 0.15 0.15 0.5] 데미지 수신, 사망처리, 사망과 시체처리
  (bind _output_get (Variables|Default|SetZombieCurrentHealth (- (Variables|Default|GetZombieCurrentHealth) Damage)))
  (if (<= _output_get (Variables|Default|GetZombieDyingHealth))
    (Utilities|ZombieDead)
    (else
      ;[0.15 0.15 0.15 0.5] 피격시 플레이어 추적
      (Variables|Default|SetbTakeDamage true)
      (Utilities|FlowControl|Delay (Variables|Default|GetTakeDamageStunTime))
      (Variables|Default|SetbTakeDamage false)
      (CallFunction|Chase))))

(fn ConstructionScript)