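; First-person player character that handles movement, look, sprint, jump, crouch, aim state and automatic rifle fire through Enhanced Input.
; BeginPlay spawns BP_Weapon on the arms' gun socket and plays the equip animation.
; Crouch timelines resize the capsule, while Tick copies control pitch to the camera Pivot.
; A DoOnce-gated Delay loop fires while CanShoot passes, spending ammo, animating the arms and messaging the weapon found by GetActorOfClass.
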(event Input|EnhancedActionEvents|EnhancedInputActionIA_Camera
  (params (ActionValue :type Vector%202D%20Structure) (ElapsedSeconds :type Float%20%28double-precision%29) (TriggeredSeconds :type Float%20%28double-precision%29) (InputAction :type Input%20Action%20Object%20Reference :default "/Game/Input/IA_Camera.IA_Camera"))
  ;[0.15 0.15 0.15 0.5] 마우스 좌우 이동으로 카메라를 좌우로 움직이기
  (:Triggered
    (bind _output_get (Variables|Default|SetMouseInput ActionValue :!label _label))
    (Pawn|Input|AddControllerYawInput (.x _output_get))
    (Pawn|Input|AddControllerPitchInput (* (.y _output_get) -1.0)))
  (:Completed
    (goto _label)))

(event Input|EnhancedActionEvents|EnhancedInputActionIA_Movement
  (params (ActionValue :type Vector%202D%20Structure) (ElapsedSeconds :type Float%20%28double-precision%29) (TriggeredSeconds :type Float%20%28double-precision%29) (InputAction :type Input%20Action%20Object%20Reference :default "/Game/Input/IA_Movement.IA_Movement"))
  ;[0.15 0.15 0.15 0.5] 내가 보는곳으로 자유롭게 이동할 수 있다
  (Pawn|Input|AddMovementInput (* (.y ActionValue) (Transformation|GetActorForwardVector)) 1.0 false)
  (Pawn|Input|AddMovementInput (* (.x ActionValue) (Transformation|GetActorRightVector)) 1.0 false))

(event Input|EnhancedActionEvents|EnhancedInputActionIA_Jump
  (params (ActionValue :type Boolean) (ElapsedSeconds :type Float%20%28double-precision%29) (TriggeredSeconds :type Float%20%28double-precision%29) (InputAction :type Input%20Action%20Object%20Reference :default "/Game/Input/IA_Jump.IA_Jump"))
  ;[0.15 0.15 0.15 0.5] 점프
  (:Triggered
    (Character|Jump))
  (:Completed
    (Character|StopJumping)))

(event Input|EnhancedActionEvents|EnhancedInputActionIA_Sprint
  (params (ActionValue :type Boolean) (ElapsedSeconds :type Float%20%28double-precision%29) (TriggeredSeconds :type Float%20%28double-precision%29) (InputAction :type Input%20Action%20Object%20Reference :default "/Game/Input/IA_Sprint.IA_Sprint"))
  ;[0.15 0.15 0.15 0.5] 달리기
  (:Triggered
    (if (not (AI|Components|NavMovement|IsFalling (Variables|Character|GetCharacterMovement)))
      (if (not (Variables|Default|GetbDoCrouching))
        (Variables|Default|SetbDoRunning true)
        (Variables|/Script/Engine.CharacterMovementComponent|SetMaxWalkSpeed (Variables|Character|GetCharacterMovement) (Variables|Default|GetRunningSpeed)))))
  (:Completed
    (if (not (AI|Components|NavMovement|IsFalling (Variables|Character|GetCharacterMovement)))
      (if (not (Variables|Default|GetbDoCrouching))
        (Variables|Default|SetbDoRunning false)
        (Variables|/Script/Engine.CharacterMovementComponent|SetMaxWalkSpeed (Variables|Character|GetCharacterMovement) (Variables|Default|GetMaxMovementSpeed))))))

(event Input|EnhancedActionEvents|EnhancedInputActionIA_Crouch
  (params (ActionValue :type Boolean) (ElapsedSeconds :type Float%20%28double-precision%29) (TriggeredSeconds :type Float%20%28double-precision%29) (InputAction :type Input%20Action%20Object%20Reference :default "/Game/Input/IA_Crouch.IA_Crouch"))
  ;[0.15 0.15 0.15 0.5] 앉기 / 앉아있다 일어나기
  (if (Variables|Default|GetbDoCrouching)
    (Variables|/Script/Engine.CharacterMovementComponent|SetMaxWalkSpeed (Variables|Character|GetCharacterMovement) (Variables|Default|GetMaxMovementSpeed))
    (bind _crouch (Timeline|TL_UnCrouch ReverseFromEnd)
      (:Update
        (CallFunction|FCrouch _crouch))
      (:Finished
        (Variables|Default|SetbDoCrouching false)))
    (else
      (Variables|/Script/Engine.CharacterMovementComponent|SetMaxWalkSpeed (Variables|Character|GetCharacterMovement) (Variables|Default|GetCrouchMovementSpeed))
      (bind _crouch_2 (Timeline|TL_Crouch PlayFromStart)
        (:Update
          (CallFunction|FCrouch _crouch_2))
        (:Finished
          (Variables|Default|SetbDoCrouching true))))))

(event Input|EnhancedActionEvents|EnhancedInputActionIA_Aim
  (params (ActionValue :type Boolean) (ElapsedSeconds :type Float%20%28double-precision%29) (TriggeredSeconds :type Float%20%28double-precision%29) (InputAction :type Input%20Action%20Object%20Reference :default "/Game/Input/IA_Aim.IA_Aim"))
  ;[0.15 0.15 0.15 0.5] 에임
  (:Triggered
    (Variables|Default|SetbDoAiming true))
  (:Completed
    (Variables|Default|SetbDoAiming false)))

(event Input|EnhancedActionEvents|EnhancedInputActionIA_Shoot
  (params (ActionValue :type Boolean) (ElapsedSeconds :type Float%20%28double-precision%29) (TriggeredSeconds :type Float%20%28double-precision%29) (InputAction :type Input%20Action%20Object%20Reference :default "/Game/Input/IA_Shoot.IA_Shoot"))
  ;[0.15 0.15 0.15 0.5] 비조준 사격
  (:Triggered
    (Utilities|FlowControl|DoOnce false :!label _label
      (:Completed
        (Variables|Default|SetbDoShooting true)
        (if (CallFunction|CanShoot) :!label _label_2
          (bind _result (Math|Integer|DecrementInt (Variables|Default|GetCurrentAmmunition))
            (:%20%20
              (Variables|Default|SetCurrentAmmunition _result)
              (Components|Animation|PlayAnimation (Variables|Default|GetPlayerArms) "/Game/Animation/A_FP_AKS74U_Fire.A_FP_AKS74U_Fire" false)
              (bind _returnvalue (Actor|GetActorOfClass "/Game/Blueprints/ForPlayer/BP_Weapon.BP_Weapon_C"))
              (Class|BIWeapon|Shoot(Message) _returnvalue)
              (Utilities|FlowControl|Delay 0.125)
              (goto _label_2)))))))
  (:Completed
    (Variables|Default|SetbDoShooting false)
    (goto _label Reset)))

(event EventTick
  (params (DeltaSeconds :type Float%20%28single-precision%29))
  ;[0.15 0.15 0.15 0.5] 위 마우스 좌우 이동과 함께 위아래 움직임 추가 (자유로운 움직임)
  (Transformation|SetRelativeRotation (Variables|Default|GetPivot) (Math|Rotator|MakeRotator 0.0 (.pitch (Pawn|GetControlRotation :!class /Script/Engine.Pawn)) 0.0) false false))

(event EventBeginPlay
  ;[0.15 0.15 0.15 0.5] 시작하자마자 총 쥐어주고 총 드는 모션 재생
  (bind _returnvalue (Game|SpawnActorfromClass "/Game/Blueprints/ForPlayer/BP_Weapon.BP_Weapon_C" (Math|Transform|MakeTransform "0, 0, 0" "0, 0, 0" "1.000000,1.000000,1.000000") "AlwaysSpawn" "MultiplyWithRoot" 0 0))
  (Transformation|AttachComponentToComponent _returnvalue (Variables|Default|GetPlayerArms) "ik_hand_gun" "KeepRelative" "KeepRelative" "KeepRelative" true)
  (Components|Animation|PlayAnimation (Variables|Default|GetPlayerArms) "/Game/Animation/A_FP_AKS74U_Equipe.A_FP_AKS74U_Equipe" false))

(fn ConstructionScript)

(fn FCrouch
  (params (Height :type Float%20%28double-precision%29))
  (Components|Capsule|SetCapsuleHalfHeight (Variables|Collision|GetCapsuleComponent) (* Height (Variables|Default|GetCapsuleHeight)) true))

(fn CanShoot
  (return (Math|Boolean|ANDBoolean (> (Variables|Default|GetCurrentAmmunition) (Variables|Default|GetEmptyAmmunition)) (Variables|Default|GetbDoShooting) (not (Variables|Default|GetbDoReloading)) (not (Variables|Default|GetbDoRunning)))))