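; BP_Weapon is a player weapon Blueprint that handles the visual side of firing and reloading.
; Shoot plays a fire animation on the Weapon mesh, attaches a scaled-down explosion emitter at FireZone as muzzle flash, then spawns a BP_Casing at the Bolt_end socket.
; Reload only plays an AKS74U reload animation.
; The graphs contain no projectile, damage or ammo-count logic.
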(event EventReload
  (Components|Animation|PlayAnimation (Variables|Default|GetWeapon) "/Game/Animation/A_WBP_AKS74U_Reload_UnEmpty.A_WBP_AKS74U_Reload_UnEmpty" false))

(event EventShoot
  ;[0.15 0.15 0.15 0.5] 사격
  (CallFunction|SetFireatGun)
  (CallFunction|AmmoShellDischarge))

(fn ConstructionScript)

(fn AmmoShellDischarge
  (bind _returnvalue (Game|SpawnActorfromClass "/Game/Blueprints/BP_Casing.BP_Casing_C" (Transformation|GetSocketTransform (Variables|Default|GetWeapon) "Bolt_end" "RTS_World") "AlwaysSpawn" "MultiplyWithRoot" 0 0))
  (Collision|IgnoreActorwhenMoving (Variables|/Game/Blueprints/BP_Casing.BP_Casing_C|GetCasingMesh _returnvalue) (Game|GetPlayerCharacter 0) false))

(fn SetFireatGun
  (bind _weapon (Variables|Default|GetWeapon))
  (Components|Animation|PlayAnimation _weapon "/Game/Animation/A_WBP_Reference_Fire.A_WBP_Reference_Fire" false)
  (Effects|SpawnEmitterAttached "/Game/StarterContent/Particles/P_Explosion.P_Explosion" _weapon "FireZone" "0, 0, 0" "0, 0, 0" "0.075000,0.075000,0.075000"))