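; BP_Zombie is an enemy character that wanders, chases the player and dies from damage.
; From BeginPlay it loops AI moves to random nearby reachable points, pausing after each successful move and retrying immediately on failure.
; An AIPerception update for the player raises walk speed to RunSpeed and starts a move toward them.
; AnyDamage lowers health; at the dying threshold the mesh ragdolls, capsule collision turns off, and the actor is destroyed after a delay.
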(event OnTargetPerceptionUpdated(AIPerception)
  (params (Actor :type Actor%20Object%20Reference) (Stimulus :type AI%20Stimulus%20Structure))
  (bind _output_get (Variables|Default|SetItMustBePlayer Actor))
  (if (== _output_get (Game|Player|GetPlayerPawn 0))
    (CallFunction|Chase)))

(event Custom|Stray
  (AI|AIMoveTo self (.RandomLocation (AI|Navigation|GetRandomReachablePointinRadius (Transformation|GetActorLocation) 5e+02 0 0)) 0 5.0 false
    (:OnSuccess
      (Utilities|FlowControl|Delay 1e+01))
    (:OnFail
      _))
  (CallFunction|Stray))

(event Custom|Chase
  (Variables|/Script/Engine.CharacterMovementComponent|SetMaxWalkSpeed (Variables|Character|GetCharacterMovement) (Variables|Default|GetRunSpeed))
  (AI|AIMoveTo self "0, 0, 0" (Variables|Default|GetItMustBePlayer) 5.0 false))

(event EventBeginPlay
  (CallFunction|Stray))

(event Game|Damage|EventAnyDamage
  (params (Damage :type Float%20%28single-precision%29) (DamageType :type Damage%20Type%20Object%20Reference) (InstigatedBy :type Controller%20Object%20Reference) (DamageCauser :type Actor%20Object%20Reference))
  (bind _mesh (Variables|Character|GetMesh))
  ;[0.15 0.15 0.15 0.5] 데미지 수신, 사망처리, 사망과 시체처리
  (bind _output_get (Variables|Default|SetZombieCurrentHealth (- (Variables|Default|GetZombieCurrentHealth) Damage)))
  (if (<= _output_get (Variables|Default|GetZombieDyingHealth))
    (Collision|SetCollisionProfileName _mesh "Ragdoll" true :!class /Script/Engine.PrimitiveComponent)
    (Physics|SetSimulatePhysics _mesh true)
    (Collision|SetCollisionEnabled (Variables|Collision|GetCapsuleComponent) "NoCollision")
    (Utilities|FlowControl|Delay 5.0)
    (Actor|DestroyActor)))

(fn ConstructionScript)