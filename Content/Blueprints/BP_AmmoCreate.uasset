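; BP_AmmoCreate is an ammo pickup actor that responds to the player's use action, though the pickup itself is not implemented yet.
; On BeginPlay it caches BP_Player and registers TakeAmmo through the player's AssignTryUseSomething.
; Box overlap events track whether that player is nearby.
; TakeAmmo checks the proximity flag, but its branch currently grants nothing.
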(event OnComponentBeginOverlap(Box)
  (params (OverlappedComponent :type Primitive%20Component%20Object%20Reference) (OtherActor :type Actor%20Object%20Reference) (OtherComp :type Primitive%20Component%20Object%20Reference) (OtherBodyIndex :type Integer) (bFromSweep :type Boolean) (SweepResult :type Hit%20Result%20Structure%20%28by%20ref%29))
  (if (== OtherActor (Variables|Default|GetAs%20BP%20Player))
    (Variables|Default|SetbIsPlayerNearby true)))

(event OnComponentEndOverlap(Box)
  (params (OverlappedComponent :type Primitive%20Component%20Object%20Reference) (OtherActor :type Actor%20Object%20Reference) (OtherComp :type Primitive%20Component%20Object%20Reference) (OtherBodyIndex :type Integer))
  (if (== (Variables|Default|GetAs%20BP%20Player) OtherActor)
    (Variables|Default|SetbIsPlayerNearby false)))

(event Custom|TakeAmmo
  (if (Variables|Default|GetbIsPlayerNearby)
    _))

(event EventBeginPlay
  (bind _asbp_player (Utilities|Casting|CastToBP_Player (Game|GetPlayerCharacter 0)))
  (bind _output_get (Variables|Default|SetAs%20BP%20Player _asbp_player))
  (EventDispatchers|AssignTryUseSomething _output_get (delegate Custom|TakeAmmo)))

(fn ConstructionScript)